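; BP_ExitGate is a level exit gate that, while open, shows the end-of-level menu when the player enters its box.
; LevelGateOpen and LevelGateClose dispatchers drive OpenGate and CloseGate, which set GateIsOpen and spawn or attempt to disable particle effects.
; Player entry spawns another effect and calls ShowEndOfLevelMenu on the cached GameInfoInstance.
; Leaving the open gate plays an exit sound, then runs a delay with nothing after it.
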(event OnComponentBeginOverlap(Box)
  (params (OverlappedComponent :type Primitive%20Component%20Object%20Reference) (OtherActor :type Actor%20Object%20Reference) (OtherComp :type Primitive%20Component%20Object%20Reference) (OtherBodyIndex :type Integer) (bFromSweep :type Boolean) (SweepResult :type Hit%20Result%20Structure%20%28by%20ref%29))
  ;[1 1 1] Players Enters the Door and Triggers Effects if LevelExit is Enabled
  (if (Variables|Default|GetGateIsOpen)
    (Utilities|Casting|CastToMyPlayerCharacter OtherActor)
    (Effects|SpawnEmitterAttached "/Game/InfinityBladeEffects/Effects/FX_Cines/Ausar/P_Ausar_Resurrection.P_Ausar_Resurrection" (Variables|Default|GetParticleSystem) "None" (Transformation|GetActorLocation) "0, 0, 0" "1.000000,1.000000,1.000000" "KeepWorldPosition")
    (Default|ShowEndOfLevelMenu (Variables|Default|GetGameInstance))))

(event OnComponentEndOverlap(Box)
  (params (OverlappedComponent :type Primitive%20Component%20Object%20Reference) (OtherActor :type Actor%20Object%20Reference) (OtherComp :type Primitive%20Component%20Object%20Reference) (OtherBodyIndex :type Integer))
  ;[1 1 1] Player Exits through Door and triggers the end of the level
  (if (Variables|Default|GetGateIsOpen)
    (Utilities|Casting|CastToMyPlayerCharacter OtherActor)
    (Audio|PlaySoundatLocation "/Game/Robotic_scifi_SFX/Voices/Robot_3/cue/phrase_exit_Cue.phrase_exit_Cue" (Transformation|GetActorLocation) "0, 0, 0" 1.0 1.0 0.0 0 0 0)
    (Utilities|FlowControl|Delay 5.0)))

(event Custom|LevelGateOpen_Event
  ;[1 1 1] Initialise and Set GameMode and GameInstance, Assign LevelGateOpen and LevelGateClose Dispatch messages
  (CallFunction|OpenGate))

(event Custom|LevelGateClose_Event
  ;[1 1 1] Initialise and Set GameMode and GameInstance, Assign LevelGateOpen and LevelGateClose Dispatch messages
  (CallFunction|CloseGate))

(event Custom|OpenGate
  ;[1 1 1] Open Level Gate, Turn on Particle Effects and Enable Level Gate
  (Effects|SpawnEmitterAttached "/Game/InfinityBladeEffects/Effects/FX_Cines/Ausar/P_Ausar_Resurrection.P_Ausar_Resurrection" (Variables|Default|GetParticleSystem) "None" (Transformation|GetActorLocation) "0, 0, 0" "1.000000,1.000000,1.000000" "KeepWorldPosition")
  (Variables|Default|SetGateIsOpen true)
  (Development|PrintString "OpenGate"))

(event Custom|CloseGate
  ;[1 1 1] Close Level Gate, Turn off Particle Effects and Disable Level Gate
  (Effects|Components|ParticleSystem|SetEmitterEnable (Variables|Default|GetParticleSystem) "None" false)
  (Variables|Default|SetGateIsOpen false)
  (Development|PrintString "Close Gate"))

(event EventBeginPlay
  ;[1 1 1] Initialise and Set GameMode and GameInstance, Assign LevelGateOpen and LevelGateClose Dispatch messages
  (bind _asmy_game_mode (Utilities|Casting|CastToMyGameMode (Game|GetGameMode)))
  (Variables|Default|SetGameMode _asmy_game_mode)
  (bind _asgame_info_instance (Utilities|Casting|CastToGameInfoInstance (Game|GetGameInstance)))
  (Variables|Default|SetGameInstance _asgame_info_instance)
  (EventDispatchers|BindEventtoLevelGateOpen (delegate Custom|LevelGateOpen_Event))
  (EventDispatchers|BindEventtoLevelGateClose (delegate Custom|LevelGateClose_Event)))

(fn ConstructionScript)

(fn CheckLevelGateIsOpen
  (if (Variables|Default|GetGateIsOpen)
    (Variables|Default|SetGateIsOpen true)
    (else
      (Variables|Default|SetGateIsOpen false))))