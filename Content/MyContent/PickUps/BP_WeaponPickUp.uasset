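; Weapon pickup actor that offers its ItemToAdd to the player while they stand in its collision volume.
; Overlap shows the pickup widget for any actor and sets AttachedWeapon on MyPlayerCharacter; end overlap hides it and clears the reference.
; A timer started at BeginPlay destroys the pickup after a minute, first decrementing AmmoSpawnCount on the PickupSpawner found in the level.
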(event OnComponentBeginOverlap(Collision)
  (params (OverlappedComponent :type Primitive%20Component%20Object%20Reference) (OtherActor :type Actor%20Object%20Reference) (OtherComp :type Primitive%20Component%20Object%20Reference) (OtherBodyIndex :type Integer) (bFromSweep :type Boolean) (SweepResult :type Hit%20Result%20Structure%20%28by%20ref%29))
  (Rendering|SetVisibility (Variables|Default|GetPickUpWidget) true false)
  (bind _asmy_player_character (Utilities|Casting|CastToMyPlayerCharacter OtherActor))
  (Variables|/Game/MyContent/Blueprints/MyPlayerCharacter.MyPlayerCharacter_C|SetAttachedWeapon _asmy_player_character (Variables|Default|GetItemToAdd)))

(event OnComponentEndOverlap(Collision)
  (params (OverlappedComponent :type Primitive%20Component%20Object%20Reference) (OtherActor :type Actor%20Object%20Reference) (OtherComp :type Primitive%20Component%20Object%20Reference) (OtherBodyIndex :type Integer))
  (Rendering|SetVisibility (Variables|Default|GetPickUpWidget) false false)
  (bind _asmy_player_character (Utilities|Casting|CastToMyPlayerCharacter OtherActor))
  (Variables|/Game/MyContent/Blueprints/MyPlayerCharacter.MyPlayerCharacter_C|SetAttachedWeapon _asmy_player_character 0))

(event EventBeginPlay
  (bind _returnvalue (Actor|GetActorOfClass "/Game/MyContent/Spawners/PickupSpawner.PickupSpawner_C"))
  (Variables|Default|SetPickupSpawnerRef _returnvalue)
  (Utilities|Time|SetTimerbyFunctionName 0 "Terminate" 6e+01))

(fn ConstructionScript)

(fn Terminate
  (Math|Integer|DecrementInt (Variables|/Game/MyContent/Spawners/PickupSpawner.PickupSpawner_C|GetAmmoSpawnCount (Variables|Default|GetPickupSpawnerRef))
    (:%20%20
      (Actor|DestroyActor))))