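; Game mode that tracks level time and Kudos score and controls whether the end-of-level gate is open.
; On BeginPlay, two looping one-second timers advance a minutes/seconds clock and recalculate Kudos.
; Each tick adds captured power points times their Kudos value, clamped to a maximum, then sets the gate-open flag once Kudos reaches that cap.
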(event EventBeginPlay
  ;[1 1 1] Start Level Timer and Kudos Counter
  (Utilities|Time|SetTimerbyFunctionName 0 "LevelTimer" 1.0 true)
  (Utilities|Time|SetTimerbyFunctionName 0 "CalculateKudos" 1.0 true))

(fn ConstructionScript)

(fn LevelTimer
  (Variables|Default|SetSeconds (+ (Variables|Default|GetSeconds) 1))
  (if (> (Variables|Default|GetSeconds) 59)
    (Variables|Default|SetMinutes (+ (Variables|Default|GetMinutes) 1))
    (Variables|Default|SetSeconds 0)))

(fn CalculateKudos
  (Variables|Default|SetKudos (Math|Integer|Clamp(Integer) (+ (Variables|Default|GetKudos) (* (Variables|Default|GetPowerPointsCaptured) (Variables|Default|GetPowerPointKudos))) 0 1000))
  (CallFunction|EnableLevelGate)
  (return))

(fn EnableLevelGate
  ;[1 1 1] Enable End of Level Gate when Kudos reaches 1000
  (if (>= (Variables|Default|GetKudos) 1000)
    (Variables|Default|SetEndOfLevelGateOpen true)
    (else
      (Variables|Default|SetEndOfLevelGateOpen false)))
  (return))