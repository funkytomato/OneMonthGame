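; Capturable power point that the player charges by standing in it, adding to the game mode's captured count when full.
; Actor overlap starts and stops a looping capture timer, while Collision component overlaps set the Capturing flag that allows Power to rise.
; A second looping timer drains Power while the point is neither captured nor being captured.
; Charging and draining play sounds, and full capture locks the point and attaches a glow emitter.
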(event OnComponentBeginOverlap(Collision)
  (params (OverlappedComponent :type Primitive%20Component%20Object%20Reference) (OtherActor :type Actor%20Object%20Reference) (OtherComp :type Primitive%20Component%20Object%20Reference) (OtherBodyIndex :type Integer) (bFromSweep :type Boolean) (SweepResult :type Hit%20Result%20Structure%20%28by%20ref%29))
  ;[1 1 1] Start Capturing
  (Utilities|Casting|CastToMyPlayerCharacter OtherActor)
  (if (not (Variables|Default|GetIsCaptured))
    (Variables|Default|SetCapturing true)))

(event OnComponentEndOverlap(Collision)
  (params (OverlappedComponent :type Primitive%20Component%20Object%20Reference) (OtherActor :type Actor%20Object%20Reference) (OtherComp :type Primitive%20Component%20Object%20Reference) (OtherBodyIndex :type Integer))
  ;[1 1 1] Stop Capturing
  (Utilities|Casting|CastToMyPlayerCharacter OtherActor)
  (Variables|Default|SetCapturing false))

(event Custom|Capture%20PowerPoint%20Event
  ;[1 1 1] Capturing Power Point
  (Utilities|FlowControl|Delay 1.0)
  (if (not (Variables|Default|GetIsCaptured))
    (if (Variables|Default|GetCapturing)
      (Variables|Default|SetPower (Math|Float|Clamp(Float) (+ (Variables|Default|GetPower) (Variables|Default|GetRechargeAmount)) 0.0 1e+02))
      (Audio|PlaySoundatLocation "/Game/GameSoundCollection/Sci-Fi_Sound_Pack_Vol_1/Cue/A_PK_HD_BoosterStart_Cue.A_PK_HD_BoosterStart_Cue" (Transformation|GetActorLocation) "0, 0, 0" 1.0 1.0 0.0 0 0 0)
      (Utilities|FlowControl|Delay 0.2)
      (if (== (Variables|Default|GetPower) 1e+02)
        (Variables|Default|SetIsCaptured true)
        (bind _asmy_game_mode (Utilities|Casting|CastToMyGameMode (Game|GetGameMode)))
        (Variables|/Game/MyContent/Blueprints/MyGameMode.MyGameMode_C|SetPowerPointsCaptured _asmy_game_mode (+ (Variables|/Game/MyContent/Blueprints/MyGameMode.MyGameMode_C|GetPowerPointsCaptured _asmy_game_mode) 1))
        (Effects|SpawnEmitterAttached "/Game/InfinityBladeEffects/Effects/FX_Cines/cinema03/P_CIN_IB_HeatGlow.P_CIN_IB_HeatGlow" (Variables|Default|GetParticleSystem) "None" (Transformation|GetActorLocation) "0, 0, 0" "5.000000,5.000000,5.000000" "KeepWorldPosition" false)))))

(event EventTick
  (params (DeltaSeconds :type Float%20%28single-precision%29)))

(event Collision|EventActorBeginOverlap
  (params (OtherActor :type Actor%20Object%20Reference))
  ;[1 1 1] Start Timer when Player enters Sphere
  (Utilities|Casting|CastToMyPlayerCharacter OtherActor)
  (Utilities|Time|SetTimerbyFunctionName 0 "Capture PowerPoint Event" 1.0 true))

(event EventBeginPlay
  ;[1 1 1] Create Timer for Reducing Power of Uncaptured Power Points
  (Utilities|Time|SetTimerbyFunctionName 0 "ReducePower" 1.0 true))

(event Collision|EventActorEndOverlap
  (params (OtherActor :type Actor%20Object%20Reference))
  ;[1 1 1] Stop Timer when Player leaves Sphere
  (Utilities|Casting|CastToMyPlayerCharacter OtherActor)
  (Utilities|Time|ClearTimerbyFunctionName 0 "Capture PowerPoint Event"))

(fn ConstructionScript)

(fn ReducePower
  (if (and (not (Variables|Default|GetIsCaptured)) (not (Variables|Default|GetCapturing)))
    (Variables|Default|SetPower (Math|Float|Clamp(Float) (- (Variables|Default|GetPower) (Variables|Default|GetRechargeAmount)) 0.0 1e+02))
    (if (> (Variables|Default|GetPower) 0.0)
      (Audio|PlaySoundatLocation "/Game/GameSoundCollection/Sci-Fi_Sound_Pack_Vol_2/Wav/P_KA_PA_Purge1.P_KA_PA_Purge1" (Transformation|GetActorLocation) "0, 0, 0" 1.0 1.0 0.0 0 0 0)
      (return))))