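; Teleport pad actor that moves the player character to a linked destination pad when they overlap its collision.
; An overlap by a player whose EnableTeleport flag is set plays a sound, then after a short delay teleports them to DestinationPad's location, using player 0's rotation.
; The flag is then cleared for TeleportTimeout seconds, blocking immediate re-teleporting by any pad that checks it.
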(event OnComponentBeginOverlap(Collision)
  (params (OverlappedComponent :type Primitive%20Component%20Object%20Reference) (OtherActor :type Actor%20Object%20Reference) (OtherComp :type Primitive%20Component%20Object%20Reference) (OtherBodyIndex :type Integer) (bFromSweep :type Boolean) (SweepResult :type Hit%20Result%20Structure%20%28by%20ref%29))
  (bind _asmy_player_character (Utilities|Casting|CastToMyPlayerCharacter OtherActor))
  (Variables|Default|SetPlayerCharacter _asmy_player_character)
  (if (Variables|/Game/MyContent/Blueprints/MyPlayerCharacter.MyPlayerCharacter_C|GetEnableTeleport _asmy_player_character)
    (CallFunction|TeleportEvent)))

(event Custom|TeleportEvent
  (bind _playercharacter (Variables|Default|GetPlayerCharacter))
  (Audio|PlaySoundatLocation "/Game/GameSoundCollection/BoardGame/Cue/ui_selest1_Cue.ui_selest1_Cue" (Transformation|GetActorLocation) "0, 0, 0" 1.0 1.0 0.0 0 0 0)
  (Utilities|FlowControl|Delay 0.2)
  (Transformation|Teleport _playercharacter (Transformation|GetActorLocation (Variables|Default|GetDestinationPad)) (Transformation|GetActorRotation (Game|GetPlayerCharacter 0)))
  (Variables|/Game/MyContent/Blueprints/MyPlayerCharacter.MyPlayerCharacter_C|SetEnableTeleport _playercharacter false)
  (Utilities|FlowControl|Delay (Variables|Default|GetTeleportTimeout))
  (Variables|/Game/MyContent/Blueprints/MyPlayerCharacter.MyPlayerCharacter_C|SetEnableTeleport _playercharacter true))

(event EventBeginPlay)

(event Collision|EventActorBeginOverlap
  (params (OtherActor :type Actor%20Object%20Reference)))

(event EventTick
  (params (DeltaSeconds :type Float%20%28single-precision%29)))

(fn ConstructionScript)